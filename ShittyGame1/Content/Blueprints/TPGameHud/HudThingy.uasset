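; HUD Blueprint that holds the game state for a timed pickup game and draws the remaining time on screen.
; StartGame runs on BeginPlay, resetting score, time, key and game-over flags, then starts a looping one-second Timer by function name.
; Timer counts time down, then sets GameOver and clears itself when time runs out.
; CoinCollected increments the score and ClockCollected adds time; only the time is drawn.
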(event `self.ReceiveDrawHUD`
  (params (SizeX :type Integer) (SizeY :type Integer))
  (`self.DrawText` (`KismetStringLibrary.Conv_IntToString` (`self.time`)) (struct :`A` 1) 10.0 10.0 null 3.0))

(event `Timer`
  ;[1 0 0.6583] Timer -- Decreases time by 1 every second and checks for Game Over
  (bind _result (`/Engine/EditorBlueprintResources/StandardMacros.DecrementInt` (`self.time`))
    (:`  `
      (if (<= _result 0)
        (set `self.gameOver` true)
        (`KismetSystemLibrary.K2_ClearTimer` null "Timer")))))

(event `self.ReceiveBeginPlay`
  (`self.startGame`))

(fn `Clock Collected`
  ;[1 1 1] Clock Collect
  (set `self.time` (+ (`self.time`) 5)))

(fn `Coin Collected`
  ;[1 1 1] Coin Collected Command
  (`/Engine/EditorBlueprintResources/StandardMacros.IncrementInt` (`self.score`)))

(fn `UserConstructionScript`)